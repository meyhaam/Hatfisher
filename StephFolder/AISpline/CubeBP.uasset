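; CubeBP is an actor that moves itself along a spline path once play begins.
; BeginPlay grabs a SplinePathBP actor from the level, then starts a timeline with its play rate set to one over TimeToCompleteInSeconds.
; Each update maps the timeline track to a distance along the spline and sets the actor's transform from world-space location and local-space rotation at that point.
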(event Custom|Move%20Object
  (bind _splineref (Variables|Default|GetSplineREF))
  (bind _spline (Variables|/Game/StephFolder/AISpline/SplinePathBP.SplinePathBP_C|GetSpline _splineref))
  (Components|Timeline|SetPlayRate (Variables|Default|GetMove%20Object%20T) (/ 1.0 (Variables|Default|GetTimeToComplete%20%28In%20Seconds%29)))
  (bind _move_track (Timeline|Move%20Object%20T Play)
    (:Update
      (Transformation|SetActorTransform (Math|Transform|MakeTransform (Spline|GetLocationatDistanceAlongSpline _spline (Math|Float|Lerp 0.0 (Spline|GetSplineLength (Variables|/Game/StephFolder/AISpline/SplinePathBP.SplinePathBP_C|GetSpline (Variables|Default|GetSplineREF))) _move_track) "World") (Spline|GetRotationatDistanceAlongSpline _spline (Math|Float|Lerp 0.0 (Spline|GetSplineLength (Variables|/Game/StephFolder/AISpline/SplinePathBP.SplinePathBP_C|GetSpline (Variables|Default|GetSplineREF))) _move_track) "Local") "1.000000,1.000000,1.000000")))))

(event EventBeginPlay
  (bind _returnvalue (Actor|GetActorOfClass "/Game/StephFolder/AISpline/SplinePathBP.SplinePathBP_C"))
  (Variables|Default|SetSplineREF _returnvalue)
  (CallFunction|MoveObject))

(fn ConstructionScript)